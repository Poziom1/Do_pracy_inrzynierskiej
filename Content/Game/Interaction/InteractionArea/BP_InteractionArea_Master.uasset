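; BP_InteractionArea_Master is a base interaction area that works through its parent actor to manage focus for character interaction.
; At BeginPlay it finds the parent's "box"-tagged shape and "interact"-tagged widget, and box overlap changes tell the other actor to reset its interaction trace.
; CanFocus can require the character to be inside the box.
; ToggleFocus notifies the parent through an interface message and shows or hides the widget.
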(event `ToggleFocus`
  (params (Focused :type Boolean))
  (bind _interactwidgetcomponentref (`self.InteractWidgetComponentRef`))
  (bind _output_get (set `self.Focused` Focused))
  (message `/Game/Game/Interaction/Bi_Interaction.Interface_ToggleFocus` (`self.GetParentActor`) _output_get)
  (`/Engine/EditorBlueprintResources/StandardMacros.IsValid` _interactwidgetcomponentref
    (:`Is Valid`
      (`SceneComponent.SetHiddenInGame` _interactwidgetcomponentref (not (`self.Focused`)) false))))

(event `self.ReceiveBeginPlay`
  (bind _output (`|GetArrayItem` (`self.GetComponentsByTag` (`self.GetParentActor`) "/Script/Engine.ShapeComponent" "box")))
  (`|ExecutionSequence`
    (:`then_0`
      (`/Engine/EditorBlueprintResources/StandardMacros.IsValid` _output
        (:`Is Valid`
          (set `self.BoxRef` _output)
          (add `PrimitiveComponent.OnComponentBeginOverlap` (`self.BoxRef`) (delegate `OnComponentBeginOverlap_Event`))
          (add `PrimitiveComponent.OnComponentEndOverlap` (`self.BoxRef`) (delegate `OnComponentEndOverlap_Event`)))))
    (:`then_1`
      (set `self.InteractWidgetComponentRef` (`|GetArrayItem` (`self.GetComponentsByTag` (`self.GetParentActor`) "/Script/UMG.WidgetComponent" "interact"))))))

(event `OnComponentBeginOverlap_Event`
  (params (OverlappedComponent :type "PrimitiveComponent Object Reference") (OtherActor :type "Actor Object Reference") (OtherComp :type "PrimitiveComponent Object Reference") (OtherBodyIndex :type Integer) (bFromSweep :type Boolean) (SweepResult :type "HitResult Structure (by ref)"))
  (message `/Game/Game/Interaction/Bi_Interaction.ResetInteractionTrace` OtherActor))

(event `OnComponentEndOverlap_Event`
  (params (OverlappedComponent :type "PrimitiveComponent Object Reference") (OtherActor :type "Actor Object Reference") (OtherComp :type "PrimitiveComponent Object Reference") (OtherBodyIndex :type Integer))
  (message `/Game/Game/Interaction/Bi_Interaction.ResetInteractionTrace` OtherActor))

(fn `CanFocus`
  (params (Charakter :type "Actor Object Reference"))
  (returns (CanFocus :type Boolean))
  (if (`self.CharakterNeedsToBeInBox`)
    (return (`PrimitiveComponent.IsOverlappingActor` (`self.BoxRef`) Charakter))
    (else
      (return true))))

(fn `UserConstructionScript`)