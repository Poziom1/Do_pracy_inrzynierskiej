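; Interaction component that lets the player focus and use interaction areas by looking at them.
; Each tick it line-traces from the camera, toggling focus on Box or CustomShape areas that pass CanFocus.
; TryToInteract fires immediately or runs a looping hold timer that fills the area's widget, cancelled on release or focus loss.
; Completion sends the interact interface message to the area's parent actor through InteractOnServer, then runs a test-print hook.
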(event `self.ReceiveTick`
  (params (DeltaSeconds :type "Float (single-precision)"))
  (`self.Trace`))

(event `TryToInteract`
  (params (In :type Boolean))
  (if In
    (if (`self.IsTrasingIteractionArea`)
      (bind _output_get (set `self.Interac Duration` (`/Game/Game/Interaction/InteractionArea/BP_InteractionArea_Master.InteracDuration` (`self.FocusedInteractionArea`))))
      (if (> _output_get 0.0)
        (bind `_aspokazanie_komętarza` (cast `/Game/Game/Pokazanie_komętarza` (`WidgetComponent.GetWidget` (`/Game/Game/Interaction/InteractionArea/BP_InteractionArea_Master.InteractWidgetComponentRef` (`self.FocusedInteractionArea`)))))
        (set `self.CurrentInteractionWidgetRef` `_aspokazanie_komętarza`)
        (bind _returnvalue (`KismetSystemLibrary.K2_SetTimerDelegate` (delegate `UpdateInteractionProgress`) (`self.UpdateInteractionInterval`) true))
        (set `self.InteractionTimer` _returnvalue)
        (else
          (`self.InteractOnServer` (`self.FocusedInteractionArea`))
          (`self.RunEventAfterInteraction`))))
    (else
      (`self.StopInteraction`))))

(event `UpdateInteractionProgress`
  (bind _output_get (set `self.InteractionProgress` (+ (`self.InteractionProgress`) (* (/ 1.0 (`self.Interac Duration`)) (`self.UpdateInteractionInterval`)))))
  (`/Game/Game/Pokazanie_komętarza.SetPrecent` (`self.CurrentInteractionWidgetRef`) _output_get)
  (if (>= (`self.InteractionProgress`) 1.0)
    (`self.StopInteraction`)
    (`self.InteractOnServer` (`self.FocusedInteractionArea`))
    (`self.RunEventAfterInteraction`)))

(event `InteractOnServer`
  (params (InteractionArea :type "/Game/Game/Interaction/InteractionArea/BP_InteractionArea_Master Object Reference"))
  (message `/Game/Game/Interaction/Bi_Interaction.InterfaceInteract` (`Actor.GetParentActor` InteractionArea)))

(fn `ReserTrace`
  (set `self.FocusetActor` null))

(fn `RunEventAfterInteraction`
  (locals (ParentActor :type "Actor Object Reference"))
  (bind _output_get (set `local.ParentActor` (`Actor.GetParentActor` (`self.FocusedInteractionArea`))))
  (if (== (`GameplayStatics.GetObjectClass` _output_get) "/Game/Game/Interaction/BP_TestInteractionActor.BP_TestInteractionActor_C")
    (`KismetSystemLibrary.PrintString` "Test")))

(fn `StopInteraction`
  (if (> (`self.InteractionProgress`) 0.0)
    (`KismetSystemLibrary.K2_ClearAndInvalidateTimerHandle` (`self.InteractionTimer`))
    (`/Game/Game/Pokazanie_komętarza.SetPrecent` (`self.CurrentInteractionWidgetRef`) 0.0)
    (set `self.InteractionProgress` 0.0)
    (set `self.CurrentInteractionWidgetRef` null)))

(fn `Trace`
  (bind _returnvalue (`GameplayStatics.GetPlayerCameraManager` 0))
  (bind _returnvalue_2 (`Actor.K2_GetActorLocation` _returnvalue))
  (bind (_outhit _returnvalue_3) (`KismetSystemLibrary.LineTraceSingle` :`Start` _returnvalue_2 :`End` (+ _returnvalue_2 (* (`KismetMathLibrary.GetForwardVector` (`Actor.K2_GetActorRotation` _returnvalue)) (`self.Length`))) :`TraceChannel` "TraceTypeQuery1" :`DrawDebugType` (`self.typ_rysowania`)))
  (if _returnvalue_3
    (bind (_bblockinghit _binitialoverlap _time _distance _location _impactpoint _normal _impactnormal _physmat _hitactor) (`GameplayStatics.BreakHitResult` _outhit))
    (if (!= (`self.FocusetActor`) _hitactor)
      (set `self.FocusetActor` _hitactor)
      (bind _returnvalue_4 (`GameplayStatics.GetObjectClass` _hitactor))
      (`self.TraceinteractionArea` (or (== _returnvalue_4 "/Game/Game/Interaction/InteractionArea/BP_InteractionArea_CustomShape.BP_InteractionArea_CustomShape_C") (== _returnvalue_4 "/Game/Game/Interaction/InteractionArea/BP_InteractionArea_Box.BP_InteractionArea_Box_C"))))
    (else
      (`self.TraceinteractionArea` false))))

(fn `TraceinteractionArea`
  (params (Trace :type Boolean))
  (if Trace
    (if (`self.IsTrasingIteractionArea`)
      (`/Game/Game/Interaction/InteractionArea/BP_InteractionArea_Master.ToggleFocus` (`self.FocusedInteractionArea`) false))
    (bind _asbp_interaction_area_master (cast `/Game/Game/Interaction/InteractionArea/BP_InteractionArea_Master` (`self.FocusetActor`)))
    (if (`/Game/Game/Interaction/InteractionArea/BP_InteractionArea_Master.CanFocus` _asbp_interaction_area_master (`self.GetOwner`))
      (bind _output_get (set `self.FocusedInteractionArea` _asbp_interaction_area_master))
      (`/Game/Game/Interaction/InteractionArea/BP_InteractionArea_Master.ToggleFocus` _output_get true)
      (set `self.IsTrasingIteractionArea` true)
      (else
        (if (`self.IsTrasingIteractionArea`) :!label _label
          (set `self.IsTrasingIteractionArea` false)
          (`/Game/Game/Interaction/InteractionArea/BP_InteractionArea_Master.ToggleFocus` (`self.FocusedInteractionArea`) false)
          (set `self.FocusetActor` null)
          (set `self.FocusedInteractionArea` null)
          (`self.StopInteraction`))))
    (else
      (goto _label))))